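; BP_Projectile is a reusable projectile actor that starts inactive and is configured and toggled through its functions, a setup suited to pooling.
; SetProperties places it and sets box extent, mesh, scale, speed and a dynamic material color.
; SetActive toggles query-only collision and visibility, and sets forward velocity to InitialSpeed or zero instead of spawning or destroying.
; Box hits are forwarded through the OnHit dispatcher, leaving the response to listeners.
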(event OnComponentHit(Box)
  (params (HitComponent :type Primitive%20Component%20Object%20Reference) (OtherActor :type Actor%20Object%20Reference) (OtherComp :type Primitive%20Component%20Object%20Reference) (NormalImpulse :type Vector :default "0, 0, 0") (Hit :type Hit%20Result%20Structure%20%28by%20ref%29))
  (Default|CallOnHit OtherActor Hit))

(event EventBeginPlay
  (CallFunction|SetActive false))

(fn ConstructionScript)

(fn SetActive
  (params (IsActive :type Boolean))
  (Collision|SetCollisionEnabled (Variables|Default|GetBox) (select IsActive "QueryOnly" "NoCollision"))
  (Rendering|SetVisibility (Variables|Default|GetStaticMesh) IsActive false)
  (Game|Components|ProjectileMovement|SetVelocityinLocalSpace (Variables|Default|GetProjectileMovement) (Math|Vector|MakeVector (* (Variables|/Script/Engine.ProjectileMovementComponent|GetInitialSpeed (Variables|Default|GetProjectileMovement)) (Math|Float|SelectFloat 1.0 0.0 IsActive)) 0.0 0.0)))

(fn SetProperties
  (params (Transform :type Transform) (ProjectileSize :type Vector :default "10.000000,10.000000,10.000000") (ProjectileScale :type Vector :default "1.000000,1.000000,1.000000") (Mesh :type Static%20Mesh%20Object%20Reference) (Material :type Material%20Instance%20Object%20Reference) (Color :type Linear%20Color%20Structure) (ProjectileSpeed :type Float%20%28single-precision%29))
  (Transformation|SetActorTransform Transform)
  (Components|Box|SetBoxExtent (Variables|Default|GetBox) ProjectileSize true)
  (Transformation|SetRelativeScale3D (Variables|Default|GetStaticMesh) ProjectileScale)
  (Components|StaticMesh|SetStaticMesh (Variables|Default|GetStaticMesh) Mesh)
  (bind _returnvalue (Rendering|Material|CreateDynamicMaterialInstance (Variables|Default|GetStaticMesh) 0 Material "None" :!class /Script/Engine.PrimitiveComponent))
  (Rendering|Material|SetVectorParameterValue _returnvalue "Color" Color :!class /Script/Engine.MaterialInstanceDynamic)
  (Variables|/Script/Engine.ProjectileMovementComponent|SetInitialSpeed (Variables|Default|GetProjectileMovement) ProjectileSpeed))