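; BP_WeaponBase is a weapon Blueprint, by name a base class, that handles automatic projectile fire.
; StartShooting sets a looping timer at the inverse of FireRate, guarded by IsShooting, though the file does not show its bound function.
; SetShootAvailable marks the weapon ready and, while IsShooting is set, calls Shoot to spawn BP_Projectile at the actor's transform.
; StopShooting only clears IsShooting, leaving the timer running.
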(event EventBeginPlay)

(fn ConstructionScript)

(fn StartShooting
  (if (not (Variables|Default|GetIsShooting))
    (bind _returnvalue (Utilities|Time|SetTimerbyEvent (EventDispatchers|CreateEvent :!event SetShootAvailable) (/ 1.0 (Variables|Default|GetFireRate)) true))
    (Variables|Default|SetShootTimer _returnvalue)
    (Variables|Default|SetIsShooting true)))

(fn StopShooting
  (Variables|Default|SetIsShooting false))

(fn SetShootAvailable
  (Variables|Default|SetIsShootAvailable true)
  (if (Variables|Default|GetIsShooting)
    (CallFunction|Shoot)))

(fn Shoot
  (Game|SpawnActorfromClass "/Game/Blueprint/Weapon/BP_Projectile.BP_Projectile_C" (Transformation|GetActorTransform) "AlwaysSpawn" 0 0))