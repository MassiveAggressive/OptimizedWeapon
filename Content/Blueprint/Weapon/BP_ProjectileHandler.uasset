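; BP_ProjectileHandler manages a pool of BP_Projectile actors and relays projectile hits through an OnHit call.
; CreateProjectilePool pre-spawns the requested number of projectiles into the Projectiles array.
; SpawnProjectile only stores the first pooled entry as the current reference.
; Its logic for setting transform, look and speed, tracking active projectiles and binding hit events is disconnected, so it never runs.
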(event Custom|OnHitEvent
  (params (OtherActor :type Actor%20Object%20Reference) (Hit :type Hit%20Result%20Structure))
  (Default|CallOnHit OtherActor Hit))

(fn ConstructionScript)

(fn SpawnProjectile
  (params (Transform :type Transform))
  (if (> (Utilities|Array|Length (Variables|Default|GetProjectiles)) 0)
    (bind _output_get (LocalVariables|SetCurrentProjectileRef (Utilities|Array|Get(acopy) (Variables|Default|GetProjectiles))))))

(fn CreateProjectilePool
  (params (Amount :type Integer))
  (for _index (range 1 Amount)
    (bind _returnvalue (Game|SpawnActorfromClass "/Game/Blueprint/Weapon/BP_Projectile.BP_Projectile_C" (Math|Transform|MakeTransform "0, 0, 0" "0, 0, 0" "1,1,1") "AlwaysSpawn" 0 0))
    (Utilities|Array|Add (Variables|Default|GetProjectiles) _returnvalue)))