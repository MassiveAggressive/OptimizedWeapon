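; BP_Player is the player pawn that moves on world axes and turns to face a hit location.
; On BeginPlay it spawns a BP_WeaponBase at Arrow1, stores it as Weapon and attaches it to that arrow component.
; Each tick it sets only its yaw toward the result of GetHitLocation, independent of movement direction.
; MoveForward and MoveRight axis inputs drive movement along fixed world X and Y.
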(event EventBeginPlay
  (bind _returnvalue (Game|SpawnActorfromClass "/Game/Blueprint/Weapon/BP_WeaponBase.BP_WeaponBase_C" (Transformation|GetWorldTransform (Variables|Default|GetArrow1)) "AlwaysSpawn" 0 0))
  (bind _output_get (Variables|Default|SetWeapon _returnvalue))
  (Transformation|AttachComponentToComponent _output_get (Variables|Default|GetArrow1) "None" "SnapToTarget" "SnapToTarget" "KeepWorld" true))

(event EventTick
  (params (DeltaSeconds :type Float%20%28single-precision%29))
  (Transformation|SetActorRotation (Math|Rotator|MakeRotator 0.0 0.0 (.yaw (Math|Rotator|FindLookatRotation (Transformation|GetActorLocation) (CallFunction|GetHitLocation))))))

(event Input|AxisEvents|InputAxisMoveForward
  (params (AxisValue :type Float%20%28single-precision%29))
  (Pawn|Input|AddMovementInput "1.000000, 0, 0" AxisValue false))

(event Input|AxisEvents|InputAxisMoveRight
  (params (AxisValue :type Float%20%28single-precision%29))
  (Pawn|Input|AddMovementInput "0,1.000000, 0" AxisValue false))

(fn ConstructionScript
  (|CallParentFunction))